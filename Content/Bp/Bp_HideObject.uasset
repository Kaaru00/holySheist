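; Actor that hides scene geometry caught in a box trace at the third-person camera, likely to keep the player's view clear.
; Each tick it traces one object type from the follow camera, sizing the box by spring arm length.
; Hit components, or their attach parents if present, are hidden with their children and recorded.
; Recorded components no longer hit are restored, removed last to first to keep indices valid.
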(event `self.ReceiveBeginPlay`
  (bind _asthird_person_character (cast `/Game/Mechanics/ThirdPersonBP/Blueprints/ThirdPersonCharacter` (`GameplayStatics.GetPlayerPawn` 0)))
  (set `self.SpringArm1` (`/Game/Mechanics/ThirdPersonBP/Blueprints/ThirdPersonCharacter.CameraBoom` _asthird_person_character))
  (set `self.Camera1` (`/Game/Mechanics/ThirdPersonBP/Blueprints/ThirdPersonCharacter.FollowCamera` _asthird_person_character))
  (`self.SetActorTickEnabled` true))

(event `self.ReceiveTick`
  (params (DeltaSeconds :type "Float (single-precision)"))
  (bind _hithidecomponent (`self.HitHideComponent`))
  (bind _indexhidecomponent (`self.IndexHideComponent`))
  (bind _returnvalue (`KismetArrayLibrary.Array_LastIndex` _indexhidecomponent))
  (bind _returnvalue_2 (`SceneComponent.GetAttachParent` (`self.SceneComponent`)))
  (bind _returnvalue_3 (`SceneComponent.K2_GetComponentLocation` (`self.Camera1`)))
  ;[0.0625 0.0625 0.0625] Hide static Mesh
  (bind _returnvalue_location (`KismetMathLibrary.BreakTransform` (`SceneComponent.GetRelativeTransform` (`/Game/Mechanics/ThirdPersonBP/Blueprints/ThirdPersonCharacter.StaticMesh` (stale `self.ReceiveBeginPlay` _asthird_person_character)))))
  (bind (_outhits _returnvalue_4) (`KismetSystemLibrary.BoxTraceMultiForObjects` _returnvalue_3 (+ _returnvalue_3 _returnvalue_location) (`KismetMathLibrary.MakeVector` 55.0 55.0 (- (`SpringArmComponent.TargetArmLength` (`self.SpringArm1`)) 100.0)) (struct :`Pitch` 30.0) (`|MakeArray` "ObjectTypeQuery7" :!type "EObjectTypeQuery Enum")))
  (if _returnvalue_4
    (`KismetArrayLibrary.Array_Clear` (`self.AllHitComponentHide`))
    (for _array_element _outhits
      (set `self.SceneComponent` (`.HitComponent` (`GameplayStatics.BreakHitResult` _array_element)))
      (`KismetArrayLibrary.Array_Add` (`self.AllHitComponentHide`) (`self.SceneComponent`))
      ;;[0.08333 0.08333 0.08333] Hide
      (if (`SceneComponent.IsVisible` (`self.SceneComponent`))
        (`/Engine/EditorBlueprintResources/StandardMacros.IsValid` _returnvalue_2
          (:`Is Valid`
            (set `self.SceneComponent` _returnvalue_2))
          (:`Is Not Valid`
            _))
        (`SceneComponent.SetVisibility` (`self.SceneComponent`) false true)
        (`KismetArrayLibrary.Array_Add` (`self.HitHideComponent`) (`self.SceneComponent`))))
    ;;[0.08333 0.08333 0.08333] Scan all hiding component and find component to unhide
    (if (`KismetArrayLibrary.Array_IsValidIndex` (`self.HitHideComponent`))
      (`KismetArrayLibrary.Array_Clear` (`self.IndexHideComponent`))
      (for (_array_element_2 _array_index) (`self.HitHideComponent`)
        (set `self.SceneComponent` _array_element_2)
        (for _array_element_3 (`self.AllHitComponentHide`)
          (bind _returnvalue_5 (`SceneComponent.GetAttachParent` _array_element_3))
          (`/Engine/EditorBlueprintResources/StandardMacros.IsValid` _returnvalue_5
            (:`Is Valid`
              (bind _returnvalue_6 (== _returnvalue_5 (`self.SceneComponent`)))
              (if _returnvalue_6
                (break)))
            (:`Is Not Valid`
              (bind _returnvalue_7 (== _array_element_3 (`self.SceneComponent`)))
              (if _returnvalue_7
                (break)))))
        (if (not (or _returnvalue_6 _returnvalue_7))
          (`KismetArrayLibrary.Array_Add` (`self.IndexHideComponent`) _array_index) ; Get index to remmove
        ))
      ;;[0.08333 0.08333 0.08333] Last To First Unhide
      (if (`KismetArrayLibrary.Array_IsValidIndex` _indexhidecomponent)
        (for _index (range (+ _returnvalue 1))
          (bind _output (`|GetArrayItem` (`self.IndexHideComponent`) (- _returnvalue _index)))
          (`SceneComponent.SetVisibility` (`|GetArrayItem` (`self.HitHideComponent`) _output) true true)
          (`KismetArrayLibrary.Array_Remove` (`self.HitHideComponent`) _output))))
    (else
      ;;[0.08333 0.08333 0.08333] All Visibility
      (if (`KismetArrayLibrary.Array_IsValidIndex` _hithidecomponent)
        (`SceneComponent.SetVisibility` _hithidecomponent true true)
        (`KismetArrayLibrary.Array_Clear` (`self.HitHideComponent`))))))

(fn `UserConstructionScript`)