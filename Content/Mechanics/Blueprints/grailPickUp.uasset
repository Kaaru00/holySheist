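; Grail pickup actor that can be interacted with or shoved by physics force.
; Interacting simply destroys the actor.
; Pushed With Force applies a randomly scaled, very large impulse to the Item, aimed from its location toward the passed Direection point.
; Older carry logic that attaches the grail to the character's ItemLocation is disconnected, and the Tick check on PickedUp does nothing.
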(event `self.ReceiveBeginPlay`)

(event `/Game/Mechanics/Blueprints/IF_Interact.Interacted`
  (params (Character :type "/Game/Mechanics/ThirdPersonBP/Blueprints/ThirdPersonCharacter Object Reference") (ComponentLocation :type "Vector Structure"))
  ;[1 1 1] monkey
  (`self.K2_DestroyActor`))

(event `Pushed with force`
  (params (direection :type "Vector Structure"))
  ;[1 1 1] MONKEY ATTEMPT WORKED
  (`PrimitiveComponent.AddImpulse` (`self.item`) (* (`KismetMathLibrary.Normal` (- direection (`SceneComponent.K2_GetComponentLocation` (`self.item`)))) (`KismetMathLibrary.RandomIntegerInRange` 100000 350000)) "None" false))

(event `self.ReceiveTick`
  (params (DeltaSeconds :type "Float (single-precision)"))
  (if (`self.PickedUp?`)
    _))

(fn `UserConstructionScript`)